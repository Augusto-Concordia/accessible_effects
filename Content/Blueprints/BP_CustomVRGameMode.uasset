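; VR game mode Blueprint that creates the Azure and accessibility manager actors when play begins.
; On BeginPlay it calls two setup functions, each spawning a manager from a class variable at the world origin and storing the instance.
; The Azure manager receives a vision options data asset and default speech options at spawn.
; Tick is disabled and the construction script only calls its parent.
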(event `self.ReceiveBeginPlay`
  (`parent.ReceiveBeginPlay`)
  (`self.SetupAzureManager`)
  (`self.SetupAccessibilityManager`))

(fn `SetupAccessibilityManager`
  (bind _returnvalue (`|SpawnActorFromClass` (`self.AccessibilityManagerClass`) (`KismetMathLibrary.MakeTransform` (0.0 0.0 0.0)) "Undefined" "MultiplyWithRoot" null null))
  (set `self.AccessibilityManagerInstance` _returnvalue))

(fn `SetupAzureManager`
  (bind _returnvalue (`|SpawnActorFromClass` (`self.AzureManagerClass`) (`KismetMathLibrary.MakeTransform` (0.0 0.0 0.0)) "Undefined" "MultiplyWithRoot" null "/Game/SeeingVR/SeeingAI/DA_AzureVisionOptions.DA_AzureVisionOptions" (`AzSpeechSettings.GetDefaultOptions`) null))
  (set `self.AzureManagerInstance` _returnvalue))

(fn `UserConstructionScript`
  (`parent.UserConstructionScript`))