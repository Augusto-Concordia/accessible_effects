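; Manager actor that toggles Highlight, Outline and Recolor post-processing effects through three referenced post-process volumes.
; BeginPlay disables all three, then Tick enables or disables each volume from its boolean flag.
; While active, Highlight turns off custom depth on static mesh actors lacking stencil 6, and Recolor turns it on, giving zero-stencil meshes random values.
; Both rescan every StaticMeshActor each frame.
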(event `self.ReceiveBeginPlay`
  (`self.RecolorOff`)
  (`self.OutlineOff`)
  (`self.HighlightOff`))

(event `self.ReceiveTick`
  (params (DeltaSeconds :type "Float (single-precision)"))
  (if (`self.highlight`)
    (`self.HighlightOn`)
    (else
      (`self.HighlightOff`)))
  (if (`self.outline`)
    (`self.OutlineOn`)
    (else
      (`self.OutlineOff`)))
  (if (`self.recolor`)
    (`self.RecolorOn`)
    (else
      (`self.RecolorOff`))))

(fn `HighlightOff`
  (bind _highlightppvolume (`self.highlightPPVolume`))
  (`/Engine/EditorBlueprintResources/StandardMacros.IsValid` _highlightppvolume
    (:`Is Valid`
      (set `PostProcessVolume.bEnabled` false _highlightppvolume))))

(fn `HighlightOn`
  (bind _highlightppvolume (`self.highlightPPVolume`))
  (`/Engine/EditorBlueprintResources/StandardMacros.IsValid` _highlightppvolume
    (:`Is Valid`
      (set `PostProcessVolume.bEnabled` true _highlightppvolume)
      (bind _outactors (`GameplayStatics.GetAllActorsOfClass` "/Script/Engine.StaticMeshActor"))
      (for _array_element _outactors
        (bind _staticmeshcomponent (`StaticMeshActor.StaticMeshComponent` _array_element))
        (if (not (== (`PrimitiveComponent.CustomDepthStencilValue` _staticmeshcomponent) 6))
          (`PrimitiveComponent.SetRenderCustomDepth` _staticmeshcomponent false))))))

(fn `OutlineOff`
  (bind _outlineppvolume (`self.outlinePPVolume`))
  (`/Engine/EditorBlueprintResources/StandardMacros.IsValid` _outlineppvolume
    (:`Is Valid`
      (set `PostProcessVolume.bEnabled` false _outlineppvolume))))

(fn `OutlineOn`
  (bind _outlineppvolume (`self.outlinePPVolume`))
  (`/Engine/EditorBlueprintResources/StandardMacros.IsValid` _outlineppvolume
    (:`Is Valid`
      (set `PostProcessVolume.bEnabled` true _outlineppvolume))))

(fn `RecolorOff`
  (bind _recolorppvolume (`self.recolorPPVolume`))
  (`/Engine/EditorBlueprintResources/StandardMacros.IsValid` _recolorppvolume
    (:`Is Valid`
      (set `PostProcessVolume.bEnabled` false _recolorppvolume))))

(fn `RecolorOn`
  (bind _recolorppvolume (`self.recolorPPVolume`))
  (`/Engine/EditorBlueprintResources/StandardMacros.IsValid` _recolorppvolume
    (:`Is Valid`
      (set `PostProcessVolume.bEnabled` true _recolorppvolume)
      (bind _outactors (`GameplayStatics.GetAllActorsOfClass` "/Script/Engine.StaticMeshActor"))
      (for _array_element _outactors
        (bind _staticmeshcomponent (`StaticMeshActor.StaticMeshComponent` _array_element))
        (if (not (`PrimitiveComponent.bRenderCustomDepth` _staticmeshcomponent))
          (`PrimitiveComponent.SetRenderCustomDepth` _staticmeshcomponent true)
          (if (== (`PrimitiveComponent.CustomDepthStencilValue` _staticmeshcomponent) 0)
            (`PrimitiveComponent.SetCustomDepthStencilValue` _staticmeshcomponent (`KismetMathLibrary.RandomIntegerInRange` 1 5))))))))

(fn `UserConstructionScript`)