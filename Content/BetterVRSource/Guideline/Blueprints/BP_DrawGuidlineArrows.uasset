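; Guideline actor that draws arrows from a point in front of the player camera to the centres of static mesh actors tagged with an AccessibleSetting component.
; BeginPlay gathers those centres and creates one ArrowComponent per centre, colored by ArrowColor.
; Tick re-aims and resizes each arrow from DistanceFromPlayer along the camera's forward vector, with visibility following IsActive.
; World-space positions are applied as relative transforms.
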(event `self.ReceiveBeginPlay`
  (bind (_returnvalue_location _returnvalue_rotation) (`KismetMathLibrary.BreakTransform` (`self.GetTransform` (`GameplayStatics.GetPlayerCameraManager` 0))))
  (bind _returnvalue (+ _returnvalue_location (* (`KismetMathLibrary.GetForwardVector` _returnvalue_rotation) (`self.distanceFromPlayer`))))
  (bind _outactors (`GameplayStatics.GetAllActorsOfClass` "/Script/Engine.StaticMeshActor"))
  (for _array_element _outactors
    (bind _returnvalue_2 (`self.K2_GetComponentsByClass` _array_element "/Game/BetterVRSource/PostProcessing/Blueprints/AccessibleSetting.AccessibleSetting_C"))
    (if (> (`KismetArrayLibrary.Array_Length` _returnvalue_2) 0)
      (`KismetArrayLibrary.Array_Add` (`self.centres`) (`/Game/BetterVRSource/PostProcessing/Blueprints/AccessibleSetting.centre` (`|GetArrayItem` _returnvalue_2)))))
  (for (_array_element_2 _array_index) (`self.centres`)
    ;[1 1 1] Create Arrows
    (bind _returnvalue_3 (`AddComponent|NODE_AddArrowComponent-4` :`RelativeTransform` (`KismetMathLibrary.MakeTransform` _returnvalue (`KismetMathLibrary.Conv_VectorToRotator` (- _array_element_2 _returnvalue)))))
    (set `ArrowComponent.ArrowLength` (`KismetMathLibrary.Vector_Distance` _returnvalue _array_element_2) _returnvalue_3)
    (set `ArrowComponent.ArrowColor` (`self.Arrow Color`) _returnvalue_3)
    (`KismetArrayLibrary.Array_Add` (`self.arrows`) _returnvalue_3)))

(event `self.ReceiveTick`
  (params (DeltaSeconds :type "Float (single-precision)"))
  (bind (_returnvalue_location _returnvalue_rotation) (`KismetMathLibrary.BreakTransform` (`self.GetTransform` (`GameplayStatics.GetPlayerCameraManager` 0))))
  (bind _returnvalue (+ _returnvalue_location (* (`KismetMathLibrary.GetForwardVector` _returnvalue_rotation) (`self.distanceFromPlayer`))))
  ;[1 1 1] Update Arrow positions
  (for (_array_element _array_index) (`self.arrows`)
    (`SceneComponent.SetVisibility` _array_element (`self.isActive`) false)
    (bind _output (`|GetArrayItem` (`self.centres`) _array_index))
    (`SceneComponent.K2_SetRelativeTransform` _array_element (`KismetMathLibrary.MakeTransform` _returnvalue (`KismetMathLibrary.Conv_VectorToRotator` (- _output _returnvalue))) false false)
    (set `ArrowComponent.ArrowLength` (`KismetMathLibrary.Vector_Distance` _returnvalue _output) _array_element)))

(fn `UserConstructionScript`)