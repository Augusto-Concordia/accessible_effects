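; BP_CycleEffects is an actor that lets the player step a post-process effect's intensity up or down through input.
; The IA_Change_Intensity_Up and IA_Change_Intensity_Down actions increment or decrement an intensity variable, with no clamping.
; Each change builds a new post-process settings struct from that value and assigns it to the PostProcess component.
; A saturation settings node and a second settings assignment remain unused.
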(event `EnhancedInput|/Game/BetterVRSource/Lenses/Input/IA_Change_Intensity_Down`
  (params (ActionValue :type Boolean) (ElapsedSeconds :type "Float (double-precision)") (TriggeredSeconds :type "Float (double-precision)") (InputAction :type "InputAction Object Reference" :default "/Game/BetterVRSource/Lenses/Input/IA_Change_Intensity_Down.IA_Change_Intensity_Down")))

(event `EnhancedInput|/Game/BetterVRSource/Lenses/Input/IA_Change_Intensity_Down`
  (params (ActionValue :type Boolean) (ElapsedSeconds :type "Float (double-precision)") (TriggeredSeconds :type "Float (double-precision)") (InputAction :type "InputAction Object Reference" :default "/Game/BetterVRSource/Lenses/Input/IA_Change_Intensity_Down.IA_Change_Intensity_Down"))
  (:`Triggered`
    (bind _result (`/Engine/EditorBlueprintResources/StandardMacros.DecrementFloat` (`self.Intesity`))
      (:`  `
        (set `PostProcessComponent.Settings` (make `PostProcessSettings` :`AutoExposureBias` _result) (`self.PostProcess`))))))

(event `EnhancedInput|/Game/BetterVRSource/Lenses/Input/IA_Change_Intensity_Up`
  (params (ActionValue :type Boolean) (ElapsedSeconds :type "Float (double-precision)") (TriggeredSeconds :type "Float (double-precision)") (InputAction :type "InputAction Object Reference" :default "/Game/BetterVRSource/Lenses/Input/IA_Change_Intensity_Up.IA_Change_Intensity_Up"))
  (:`Triggered`
    (bind _result (`/Engine/EditorBlueprintResources/StandardMacros.IncrementFloat` (`self.Intesity`))
      (:`  `
        (set `PostProcessComponent.Settings` (make `PostProcessSettings` :`AutoExposureBias` _result) (`self.PostProcess`))))))

(fn `UserConstructionScript`)