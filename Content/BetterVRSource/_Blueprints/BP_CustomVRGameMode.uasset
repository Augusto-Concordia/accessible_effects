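; VR game mode that sets up the Azure and accessibility managers when play begins.
; Spawns the Azure manager at the world origin with a vision options data asset and default speech options, then stores the instance.
; Looks up and caches the accessibility manager already placed in the level, printing an error and quitting the game if none is found.
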(event `self.ReceiveBeginPlay`
  (`parent.ReceiveBeginPlay`)
  (`self.SetupAzureManager`)
  (`self.SetupAccessibilityManager`))

(fn `SetupAccessibilityManager`
  (bind _returnvalue (`GameplayStatics.GetActorOfClass` (`self.AccessibilityManagerClass`)))
  (if (`KismetSystemLibrary.IsValid` _returnvalue)
    (set `self.AccessibilityManagerInstance` _returnvalue)
    (else
      (`KismetSystemLibrary.PrintString` "Could not find Accessibility Manager in level!" true true (struct :`G` 0.66 :`B` 1.0 :`A` 1.0) 5.0)
      (`KismetSystemLibrary.QuitGame` null "Quit"))))

(fn `SetupAzureManager`
  (bind _returnvalue (`|SpawnActorFromClass` (`self.AzureManagerClass`) (`KismetMathLibrary.MakeTransform` (0.0 0.0 0.0)) "Undefined" "MultiplyWithRoot" null "/Game/BetterVRSource/SeeingAI/DA_AzureVisionOptions.DA_AzureVisionOptions" (`AzSpeechSettings.GetDefaultOptions`) null))
  (set `self.AzureManagerInstance` _returnvalue))

(fn `UserConstructionScript`
  (`parent.UserConstructionScript`))