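; Accessibility manager that toggles text augmentation and selects a lens tool through Enhanced Input actions.
; It caches all BP_AccessibleTextRender actors at construction and BeginPlay, then pushes the augmentation state to each on toggle or construction.
; Next and previous inputs step CurrentTool with a hardcoded modulo of ten.
; SetCurrentLens shows only the matching ToolActors entry, though no graph here calls it.
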(event `self.ReceiveBeginPlay`
  (`EnhancedInputSubsystemInterface.AddMappingContext` (pcsubsystem `EnhancedInputLocalPlayerSubsystem` (`GameplayStatics.GetPlayerController` 0)) "/Game/BetterVRSource/_Input/IMC_AccessibleActions.IMC_AccessibleActions" 0 (struct))
  (`self.CollectAllRenderTexts`))

(event `EnhancedInput|/Game/BetterVRSource/_Input/IA_ToggleTextAugmentation`
  (params (ActionValue :type Boolean) (ElapsedSeconds :type "Float (double-precision)") (TriggeredSeconds :type "Float (double-precision)") (InputAction :type "InputAction Object Reference" :default "/Game/BetterVRSource/_Input/IA_ToggleTextAugmentation.IA_ToggleTextAugmentation"))
  (:`Started`
    (`self.UpdateRenderTexts` (not (`self.AreTextsAugmented`)))))

(event `EnhancedInput|/Game/BetterVRSource/_Input/IA_NextLens`
  (params (ActionValue :type Boolean) (ElapsedSeconds :type "Float (double-precision)") (TriggeredSeconds :type "Float (double-precision)") (InputAction :type "InputAction Object Reference" :default "/Game/BetterVRSource/_Input/IA_NextLens.IA_NextLens"))
  (:`Started`
    (set `self.CurrentTool` (mod (+ (`self.CurrentTool`) 1) 10))))

(event `EnhancedInput|/Game/BetterVRSource/_Input/IA_PreviousLens`
  (params (ActionValue :type Boolean) (ElapsedSeconds :type "Float (double-precision)") (TriggeredSeconds :type "Float (double-precision)") (InputAction :type "InputAction Object Reference" :default "/Game/BetterVRSource/_Input/IA_PreviousLens.IA_PreviousLens"))
  (:`Started`
    (set `self.CurrentTool` (mod (+ (`self.CurrentTool`) -1) 10))))

(fn `CollectAllRenderTexts`
  (bind _outactors (`GameplayStatics.GetAllActorsOfClass` "/Game/BetterVRSource/TTS/Blueprints/BP_AccessibleTextRender.BP_AccessibleTextRender_C"))
  (set `self.FoundAccessibleTextRenders` _outactors)
  (return))

(fn `SetCurrentLens`
  (for (_array_element _array_index) (`self.ToolActors`)
    (`self.SetActorHiddenInGame` _array_element (not (== _array_index (`self.CurrentTool`))))))

(fn `UpdateRenderTexts`
  (params (ShouldTextsBeAugmented :type Boolean))
  (bind _output_get (set `self.AreTextsAugmented` ShouldTextsBeAugmented))
  (for _array_element (`self.FoundAccessibleTextRenders`)
    (`/Game/BetterVRSource/TTS/Blueprints/BP_AccessibleTextRender.SetTextAugmentation` _array_element _output_get)))

(fn `UserConstructionScript`
  (`self.CollectAllRenderTexts`)
  (`self.UpdateRenderTexts` (`self.AreTextsAugmented`)))