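; Manager Blueprint that turns queued text into speech through Azure text-to-speech and plays it as 2D sound.
; QueueTTSText appends to a queue, and Tick processes the front entry, playing a cached sound or starting async synthesis with the current Azure options.
; Entries leave the queue without waiting for synthesis or playback, so lines can overlap.
; Completed sounds play and are optionally cached by text; failures only print in debug.
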(event `self.ReceiveTick`
  (params (DeltaSeconds :type "Float (single-precision)"))
  (`self.ProcessTTSQueue`))

(fn `QueueTTSText`
  (params (Input :type Text))
  (`KismetArrayLibrary.Array_Add` (`self.TTSQueue`) Input)
  (return))

(fn `UserConstructionScript`)