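; BP_TTSTextFinder is an actor that finds text in the world along its forward vector and sends it for text-to-speech.
; Each tick it line-traces up to FindRange for a BP_FindableTextRender.
; When the found object changes, it queues that text on the Azure manager held by BP_CustomVRGameMode.
; In debug mode it prints the text and moves HitPoint to the hit location.
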(event `self.ReceiveTick`
  (params (DeltaSeconds :type "Float (single-precision)"))
  (bind (_foundfindabletext _foundtext) (`self.LineTraceForText`))
  ;[0 0 0] Guarantees that only new pieces of text are sent for TTS
  (if (not (== (`self.LastFoundFindableText`) _foundfindabletext))
    (bind _output_get (set `self.LastFoundFindableText` _foundfindabletext))
    (if (`KismetSystemLibrary.IsValid` _output_get)
      (bind _asbp_custom_vrgame_mode (cast `/Game/Blueprints/BP_CustomVRGameMode` (`GameplayStatics.GetGameMode`)))
      (`/Engine/EditorBlueprintResources/StandardMacros.IsValid` _asbp_custom_vrgame_mode
        (:`Is Valid`
          (`/Game/TTS/Blueprints/BP_AzureManager.QueueTTSText` (`/Game/Blueprints/BP_CustomVRGameMode.AzureManagerInstance` _asbp_custom_vrgame_mode) _foundtext))
        (:`Is Not Valid`
          (`KismetSystemLibrary.PrintString` "Could not get current custom VR game mode"))))))

(fn `LineTraceForText`
  (returns (FoundFindableText :type "/Game/TTS/Blueprints/BP_FindableTextRender Object Reference") (FoundText :type Text))
  (bind _returnvalue (`self.K2_GetActorLocation`))
  (bind _outhit (`KismetSystemLibrary.LineTraceSingleForObjects` _returnvalue (+ _returnvalue (* (`self.FindRange`) (`self.GetActorForwardVector`))) (`|MakeArray` "ObjectTypeQuery2" "ObjectTypeQuery1" :!type "EObjectTypeQuery Enum")))
  (bind (_bblockinghit _binitialoverlap _time _distance _location _impactpoint _normal _impactnormal _physmat _hitactor) (`GameplayStatics.BreakHitResult` _outhit))
  (bind _asbp_findable_text_render (cast `/Game/TTS/Blueprints/BP_FindableTextRender` _hitactor)
    (:`then`
      (bind _textasstring (`/Game/TTS/Blueprints/BP_FindableTextRender.Get Text` _asbp_findable_text_render))
      (if (`self.Is Debug`)
        (`KismetSystemLibrary.PrintText` _textasstring true true (struct :`G` 0.66 :`B` 1.0 :`A` 1.0) 2.0 "LTfT")
        (`SceneComponent.K2_SetWorldLocation` (`self.HitPoint`) _location false false)
        (return _asbp_findable_text_render _textasstring)
        (else
          (return _asbp_findable_text_render _textasstring))))
    (:`CastFailed`
      (`SceneComponent.K2_SetRelativeLocation` (`self.HitPoint`) (0.0 0.0 0.0) false false)
      (return null "") ; If we haven't found anything that is valid, just return null
    )))

(fn `UserConstructionScript`)