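; Data asset holding Azure Vision request options for the SeeingAI feature of SeeingVR.
; It stores the endpoint, API version, subscription key and analysis parameters such as features, model, language and captioning options.
; One function exposes all fields as separate outputs, and another reuses it to pack them into an AzureVisionSettings struct.
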(fn `BreakAzureVisionOptions`
  (returns (BaseUrl :type String) (ApiVersion :type String) (Features :type String) (ModelName :type String) (Language :type String) (SmartCropsAspectRatios :type String) (GenderNeutralCaption :type Boolean) (OcpApimSubscriptionKey :type String))
  (return (`self.BaseUrl`) (`self.ApiVersion`) (`self.Features`) (`self.ModelName`) (`self.Language`) (`self.SmartCropsAspectRatios`) (`self.GenderNeutralCaption`) (`self.OcpApimSubscriptionKey`)))

(fn `ToAzureVisionOptionsStruct`
  (returns (AzureVisionSettings :type "AzureVisionSettings Structure"))
  (bind (_baseurl _apiversion _features _modelname _language _smartcropsaspectratios _genderneutralcaption _ocpapimsubscriptionkey) (`self.BreakAzureVisionOptions`))
  (return (make `AzureVisionSettings` _baseurl _apiversion _features _modelname _language _smartcropsaspectratios _genderneutralcaption _ocpapimsubscriptionkey)))