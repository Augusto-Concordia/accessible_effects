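; SeeingVR scene-captioning Blueprint that sends the player's view to an Azure vision service on demand.
; A SceneCaptureComponent2D follows the player camera every Tick, with its render target sized to half the viewport at BeginPlay.
; IA_CaptionScene triggers a capture, then RequestSceneCaptions reads the pixels, encodes them as PNG and passes them to the custom VR game mode's AzureManagerInstance.
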(event `EnhancedInput|/Game/SeeingVR/SeeingAI/Input/IA_CaptionScene`
  (params (ActionValue :type Boolean) (ElapsedSeconds :type "Float (double-precision)") (TriggeredSeconds :type "Float (double-precision)") (InputAction :type "InputAction Object Reference" :default "/Game/SeeingVR/SeeingAI/Input/IA_CaptionScene.IA_CaptionScene"))
  (:`Started`
    (`SceneCaptureComponent2D.CaptureScene` (`self.SceneCaptureComponent2D`))
    (bind _asbp_custom_vrgame_mode (cast `/Game/Blueprints/BP_CustomVRGameMode` (`GameplayStatics.GetGameMode`)))
    (`/Engine/EditorBlueprintResources/StandardMacros.IsValid` _asbp_custom_vrgame_mode
      (:`Is Valid`
        (`self.RequestSceneCaptions` (`/Game/Blueprints/BP_CustomVRGameMode.AzureManagerInstance` _asbp_custom_vrgame_mode)))
      (:`Is Not Valid`
        (`KismetSystemLibrary.PrintString` "Could not get current custom VR game mode")))))

(event `self.ReceiveBeginPlay`
  (bind (_returnvalue_x _returnvalue_y) (`KismetMathLibrary.BreakVector2D` (/ (`WidgetLayoutLibrary.GetViewportSize`) (2.0 2.0))))
  (set `self.MainCamera` (`self.GetComponentByClass` (`GameplayStatics.GetPlayerPawn` 0) "/Script/Engine.CameraComponent"))
  (`GameUserSettings.GetGameUserSettings`)
  (`KismetRenderingLibrary.ResizeRenderTarget2D` (`self.SceneRenderTarget`) (`KismetMathLibrary.FTrunc` _returnvalue_x) (`KismetMathLibrary.FTrunc` _returnvalue_y)))

(event `self.ReceiveTick`
  (params (DeltaSeconds :type "Float (single-precision)"))
  (`SceneComponent.K2_SetWorldTransform` (`self.SceneCaptureComponent2D`) (`SceneComponent.K2_GetComponentToWorld` (`self.MainCamera`)) false false))

(fn `RequestSceneCaptions`
  (params (`Azure Manager Instance` :type "/Game/SeeingVR/_Blueprints/BP_AzureManager2 Object Reference (by ref)"))
  (locals (ImageDataArray :type "Array of Byte"))
  (bind _scenerendertarget (`self.SceneRenderTarget`))
  (bind _outsamples (`KismetRenderingLibrary.ReadRenderTarget` _scenerendertarget))
  (bind _returnvalue (`FUtilities.GetImagePixelsInPNG` (`TextureRenderTarget2D.SizeX` _scenerendertarget) (`TextureRenderTarget2D.SizeY` _scenerendertarget) _outsamples))
  (`/Game/SeeingVR/_Blueprints/BP_AzureManager2.ProcessVisionRequest` `Azure Manager Instance` _returnvalue)
  (return))

(fn `UserConstructionScript`)