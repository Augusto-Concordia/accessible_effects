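; BP_AccessibilityManager is a SeeingVR manager that toggles text augmentation across all BP_AccessibleTextRender actors in the level.
; It caches those actors in the construction script and again on BeginPlay, where it also adds the IMC_AccessibleActions input mapping context.
; The IA_ToggleTextAugmentation input flips AreTextsAugmented and passes the new state to each cached actor.
; The construction script also applies the current state, so it takes effect without play starting.
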(event `self.ReceiveBeginPlay`
  (`EnhancedInputSubsystemInterface.AddMappingContext` (pcsubsystem `EnhancedInputLocalPlayerSubsystem` (`GameplayStatics.GetPlayerController` 0)) "/Game/SeeingVR/TextAugmentation/Input/IMC_AccessibleActions.IMC_AccessibleActions" 0 (struct))
  (`self.CollectAllRenderTexts`))

(event `EnhancedInput|/Game/SeeingVR/TextAugmentation/Input/IA_ToggleTextAugmentation`
  (params (ActionValue :type Boolean) (ElapsedSeconds :type "Float (double-precision)") (TriggeredSeconds :type "Float (double-precision)") (InputAction :type "InputAction Object Reference" :default "/Game/SeeingVR/TextAugmentation/Input/IA_ToggleTextAugmentation.IA_ToggleTextAugmentation"))
  (:`Triggered`
    (`self.UpdateRenderTexts` (not (`self.AreTextsAugmented`)))))

(fn `CollectAllRenderTexts`
  (bind _outactors (`GameplayStatics.GetAllActorsOfClass` "/Game/SeeingVR/TTS/Blueprints/BP_AccessibleTextRender.BP_AccessibleTextRender_C"))
  (set `self.FoundAccessibleTextRenders` _outactors)
  (return))

(fn `UpdateRenderTexts`
  (params (ShouldTextsBeAugmented :type Boolean))
  (bind _output_get (set `self.AreTextsAugmented` ShouldTextsBeAugmented))
  (for _array_element (`self.FoundAccessibleTextRenders`)
    (`/Game/SeeingVR/TTS/Blueprints/BP_AccessibleTextRender.SetTextAugmentation` _array_element _output_get)))

(fn `UserConstructionScript`
  (`self.CollectAllRenderTexts`)
  (`self.UpdateRenderTexts` (`self.AreTextsAugmented`)))