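; SeeingVR manager Blueprint for Azure text-to-speech, with an unfinished vision request stub.
; QueueTTSText adds text to a queue that Tick processes one entry at a time.
; Cached lines play immediately as 2D sound; others go to async Azure synthesis, play on completion and are optionally cached by text.
; Entries leave the queue when synthesis starts, so requests can overlap, and failures only print a message.
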(event `self.ReceiveTick`
  (params (DeltaSeconds :type "Float (single-precision)"))
  (`self.ProcessTTSQueue`))

(fn `ProcessVisionRequest`
  (params (ImageData :type "Array of Byte"))
  (`/Game/SeeingVR/SeeingAI/Blueprints/BDA_AzureVisionOptions.ToAzureVisionOptionsStruct` (`self.CurrentAzureVisionOptions`)))

(fn `QueueTTSText`
  (params (Input :type Text))
  (`KismetArrayLibrary.Array_Add` (`self.TTSQueue`) Input)
  (return))

(fn `UserConstructionScript`)