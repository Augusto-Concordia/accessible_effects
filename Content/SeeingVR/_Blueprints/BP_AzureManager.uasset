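; Azure manager for SeeingVR that captions image data with Azure Vision and reads the captions aloud through Azure Speech.
; ProcessVisionRequest requests dense captions, and successful results join a TTS queue while failures are printed.
; Each tick handles the head of the queue, playing cached audio or starting async synthesis without waiting for earlier sounds to finish.
; New sounds are cached by text when caching is enabled.
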(event `self.ReceiveTick`
  (params (DeltaSeconds :type "Float (single-precision)"))
  (`self.ProcessTTSQueue`))

(event `OnVisionSuccess`
  (params (Caption :type String))
  (`self.QueueTTSText` (`KismetTextLibrary.Conv_StringToText` Caption)))

(event `OnVisionFailure`
  (params (Msg :type String))
  (`KismetSystemLibrary.PrintString` Msg))

(fn `ProcessVisionRequest`
  (params (ImageData :type "Array of Byte"))
  (bind _azurevisionsettings (`/Game/SeeingVR/SeeingAI/Blueprints/BDA_AzureVisionOptions.ToAzureVisionOptionsStruct` (`self.CurrentAzureVisionOptions`)))
  (`FAzureVision.GetImageDenseCaptions` _azurevisionsettings ImageData (`|CreateDelegate` :!event `OnVisionSuccess`) (`|CreateDelegate` :!event `OnVisionFailure`))
  (return))

(fn `QueueTTSText`
  (params (Input :type Text))
  (`KismetArrayLibrary.Array_Add` (`self.TTSQueue`) Input)
  (return))

(fn `UserConstructionScript`)