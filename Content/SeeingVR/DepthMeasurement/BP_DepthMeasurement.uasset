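; BP_DepthMeasurement is a SeeingVR depth aid that draws a line from the actor to the first object ahead of it.
; Each Tick, CustomLineTrace runs an object-type trace along the forward vector up to FindRange.
; SetLineAndSphere moves the HitPoint marker and feeds Niagara line endpoints, collapsing them to world origin on a miss.
; HitPoint shows only on a hit with IsSphereVisible set; an unused UMG line attempt remains unwired.
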(event `self.ReceiveBeginPlay`)

(event `self.ReceiveTick`
  (params (DeltaSeconds :type "Float (single-precision)"))
  (bind (_validhit _location) (`self.CustomLineTrace`))
  (`SceneComponent.SetVisibility` (`self.HitPoint`) (and (`self.IsSphereVisible`) _validhit) true)
  (if _validhit
    (`self.SetLineAndSphere` (`self.K2_GetActorLocation`) _location)
    (else
      (`self.SetLineAndSphere` (0.0 0.0 0.0)))))

(fn `CustomLineTrace`
  (returns (ValidHit :type Boolean) (Location :type "Vector Structure") (HitActor :type "Actor Object Reference") (HitActorComponent :type "ActorComponent Object Reference"))
  (bind _returnvalue (`self.K2_GetActorLocation`))
  (bind (_outhit _returnvalue_2) (`KismetSystemLibrary.LineTraceSingleForObjects` _returnvalue (+ _returnvalue (* (`self.FindRange`) (`self.GetActorForwardVector`))) (`|MakeArray` "ObjectTypeQuery2" "ObjectTypeQuery1" "ObjectTypeQuery4" "ObjectTypeQuery3" "ObjectTypeQuery5" "ObjectTypeQuery6" :!type "EObjectTypeQuery Enum")))
  (bind (_bblockinghit _binitialoverlap _time _distance _location _impactpoint _normal _impactnormal _physmat _hitactor _hitcomponent) (`GameplayStatics.BreakHitResult` _outhit))
  (return _returnvalue_2 _location _hitactor _hitcomponent))

(fn `SetLineAndSphere`
  (params (Start :type "Vector Structure") (End :type "Vector Structure"))
  (bind _output_get (set `self.LineStart` Start))
  (bind _output_get_2 (set `self.LineEnd` End))
  (`SceneComponent.K2_SetWorldLocation` (`self.HitPoint`) _output_get_2 false false)
  (`self.SetNiagaraLineEndpoints` _output_get _output_get_2))

(fn `SetNiagaraLineEndpoints`
  (params (Start :type "Vector Structure") (End :type "Vector Structure"))
  (bind _ns_depthline (`self.NS_DepthLine`))
  (`FXSystemComponent.SetVectorParameter` _ns_depthline "User.LineStart" Start)
  (`FXSystemComponent.SetVectorParameter` _ns_depthline "User.LineEnd" End))

(fn `UserConstructionScript`)