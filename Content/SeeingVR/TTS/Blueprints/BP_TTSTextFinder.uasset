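; BP_TTSTextFinder detects findable in-world text along its line of sight and sends it to text-to-speech as part of SeeingVR.
; On BeginPlay it spawns an attached, invisible BP_DepthMeasurement to supply hit results.
; Each tick it checks whether the hit actor is a BP_FindableTextRender and, only when that target changes, queues its text on the custom VR game mode's Azure manager.
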(event `self.ReceiveBeginPlay`
  (bind _returnvalue (`|SpawnActorFromClass` "/Game/SeeingVR/DepthMeasurement/Blueprints/BP_DepthMeasurement.BP_DepthMeasurement_C" (`self.GetTransform`) "Undefined" "MultiplyWithRoot" self (`self.FindRange`) false null))
  (bind _output_get (set `self.DepthMeasurementInstance` _returnvalue))
  (`self.K2_AttachToActor` _output_get self "None" "SnapToTarget" "SnapToTarget" "SnapToTarget" true))

(event `self.ReceiveTick`
  (params (DeltaSeconds :type "Float (single-precision)"))
  (bind (_foundfindabletext _foundtext) (`self.LineTraceForText`))
  ;[0 0 0] Guarantees that only new pieces of text are sent for TTS
  (if (not (== (`self.LastFoundFindableText`) _foundfindabletext))
    (bind _output_get (set `self.LastFoundFindableText` _foundfindabletext))
    (if (`KismetSystemLibrary.IsValid` _output_get)
      (bind _asbp_custom_vrgame_mode (cast `/Game/Blueprints/BP_CustomVRGameMode` (`GameplayStatics.GetGameMode`)))
      (`/Engine/EditorBlueprintResources/StandardMacros.IsValid` _asbp_custom_vrgame_mode
        (:`Is Valid`
          (`/Game/SeeingVR/TTS/Blueprints/BP_AzureManager.QueueTTSText` (`/Game/Blueprints/BP_CustomVRGameMode.AzureManagerInstance` _asbp_custom_vrgame_mode) _foundtext))
        (:`Is Not Valid`
          (`KismetSystemLibrary.PrintString` "Could not get current custom VR game mode"))))))

(fn `LineTraceForText`
  (returns (FoundFindableText :type "/Game/SeeingVR/TTS/Blueprints/BP_FindableTextRender Object Reference") (FoundText :type Text))
  (bind (_linestart _lineend _hitactor) (`/Game/SeeingVR/DepthMeasurement/Blueprints/BP_DepthMeasurement.GetHitInformation` (`self.DepthMeasurementInstance`)))
  (bind _asbp_findable_text_render (cast `/Game/SeeingVR/TTS/Blueprints/BP_FindableTextRender` _hitactor)
    (:`then`
      (bind _textasstring (`/Game/SeeingVR/TTS/Blueprints/BP_FindableTextRender.Get Text` _asbp_findable_text_render))
      (return _asbp_findable_text_render _textasstring))
    (:`CastFailed`
      (return null "") ; If we haven't found anything that is valid, just return null
    )))

(fn `UserConstructionScript`)