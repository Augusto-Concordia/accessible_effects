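; BP_AccessibleTextRender is a text render actor for the SeeingVR text-to-speech and text augmentation accessibility feature.
; The construction script sizes LineTraceBox from half the text's local size, giving the text a matching box extent.
; GetText exposes the displayed string to callers.
; SetTextAugmentation stores a flag and switches the text material between the default and an augmented opaque one, which construction also applies.
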(fn `Get Text`
  (returns (TextAsString :type Text))
  (return (`TextRenderComponent.Text` (`self.TextRender`))))

(fn `SetTextAugmentation`
  (params (ShouldTextBeAugmented :type Boolean))
  (set `self.IsTextAugmented` ShouldTextBeAugmented)
  (`self.UpdateAugmentationMaterial`))

(fn `UpdateAugmentationMaterial`
  (locals (NewMaterial :type "Material Object Reference"))
  (if (`self.IsTextAugmented`)
    (set `local.NewMaterial` "/Game/SeeingVR/TextAugmentation/Materials/M_AugmentedOpaqueText.M_AugmentedOpaqueText")
    (else
      (set `local.NewMaterial` (`self.DefaultMaterial`))))
  (`PrimitiveComponent.SetMaterial` (`self.TextRender`) 0 (`local.NewMaterial`))
  (return))

(fn `UserConstructionScript`
  (`BoxComponent.SetBoxExtent` (`self.Line Trace Box`) (/ (`TextRenderComponent.GetTextLocalSize` (`self.TextRender`)) (2.0 2.0 2.0)) true)
  (`self.UpdateAugmentationMaterial`))