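; BP_TTSAgent reads aloud, via text-to-speech, text and object descriptions its depth probe hits in VR.
; It spawns and attaches a BP_DepthMeasurement actor, then each tick checks the hit actor for BP_AccessibleTextRender text or a BP_ObjectDescription component.
; A per-source cache of last found strings lets only changed, non-empty text reach the game mode's AzureManager TTS queue.
; Empty results reset the cache, so revisited text is queued again.
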(event `self.ReceiveBeginPlay`
  (bind _returnvalue (`|SpawnActorFromClass` "/Game/SeeingVR/DepthMeasurement/Blueprints/BP_DepthMeasurement.BP_DepthMeasurement_C" (`self.GetTransform`) "Undefined" "MultiplyWithRoot" self (`self.FindRange`) false null))
  (bind _output_get (set `self.DepthMeasurementInstance` _returnvalue))
  (`self.K2_AttachToActor` _output_get self "None" "SnapToTarget" "SnapToTarget" "SnapToTarget" true))

(event `self.ReceiveTick`
  (params (DeltaSeconds :type "Float (single-precision)"))
  (bind (_foundfindabletext _foundtext) (`self.LineTraceForText`))
  (bind (_objectdescription _foundtext_2) (`self.LineTraceForDescriptions`))
  (for (_array_element _array_index) (`|MakeArray` _foundtext_2 _foundtext)
    (bind _returnvalue (`KismetTextLibrary.Conv_TextToString` _array_element))
    (if (`KismetStringLibrary.IsEmpty` _returnvalue)
      ;[0 0 0] If the string is empty, save it, but don't send it to TTS
      (`BlueprintMapLibrary.Map_Add` (`self.LastFoundStrings`) _array_index)
      (else
        ;[0 0 0] Guarantees that only new pieces of text are sent for TTS
        (if (not (`KismetStringLibrary.EqualEqual_StrStr` (`BlueprintMapLibrary.Map_Find` (`self.LastFoundStrings`) _array_index) _returnvalue))
          (`BlueprintMapLibrary.Map_Add` (`self.LastFoundStrings`) _array_index _returnvalue)
          (bind _asbp_custom_vrgame_mode (cast `/Game/Blueprints/BP_CustomVRGameMode` (`GameplayStatics.GetGameMode`)))
          (`/Engine/EditorBlueprintResources/StandardMacros.IsValid` _asbp_custom_vrgame_mode
            (:`Is Valid`
              (`/Game/SeeingVR/_Blueprints/BP_AzureManager2.QueueTTSText` (`/Game/Blueprints/BP_CustomVRGameMode.AzureManagerInstance` _asbp_custom_vrgame_mode) _array_element))
            (:`Is Not Valid`
              (`KismetSystemLibrary.PrintString` "Could not get current custom VR game mode"))))))))

(fn `LineTraceForDescriptions`
  (returns (ObjectDescription :type "/Game/SeeingVR/ObjectDescription/Blueprints/BP_ObjectDescription Object Reference") (FoundText :type Text))
  (bind (_linestart _lineend _hitactor) (`/Game/SeeingVR/DepthMeasurement/Blueprints/BP_DepthMeasurement.GetHitInformation` (`self.DepthMeasurementInstance`)))
  (if (`KismetSystemLibrary.IsValid` _hitactor)
    (bind _returnvalue (`self.GetComponentByClass` _hitactor "/Game/SeeingVR/ObjectDescription/Blueprints/BP_ObjectDescription.BP_ObjectDescription_C"))
    (if (`KismetSystemLibrary.IsValid` _returnvalue)
      (return _returnvalue (`/Game/SeeingVR/ObjectDescription/Blueprints/BP_ObjectDescription.Description` _returnvalue))
      (else
        (return null "")))
    (else
      (return null ""))))

(fn `LineTraceForText`
  (returns (FoundFindableText :type "/Game/SeeingVR/TTS/Blueprints/BP_AccessibleTextRender Object Reference") (FoundText :type Text))
  (bind (_linestart _lineend _hitactor) (`/Game/SeeingVR/DepthMeasurement/Blueprints/BP_DepthMeasurement.GetHitInformation` (`self.DepthMeasurementInstance`)))
  (bind _asbp_accessible_text_render (cast `/Game/SeeingVR/TTS/Blueprints/BP_AccessibleTextRender` _hitactor)
    (:`then`
      (bind _textasstring (`/Game/SeeingVR/TTS/Blueprints/BP_AccessibleTextRender.Get Text` _asbp_accessible_text_render))
      (return _asbp_accessible_text_render _textasstring))
    (:`CastFailed`
      (return null "") ; If we haven't found anything that is valid, just return null
    )))

(fn `UserConstructionScript`)